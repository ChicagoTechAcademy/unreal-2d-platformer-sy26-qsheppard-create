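; Player character Blueprint for the Satyr, with movement along the world X axis and jumping.
; On BeginPlay it adds the Satyr Enhanced Input mapping context to the local player's subsystem.
; Move input is rounded and applied as X-axis movement, after RotateController snaps control yaw forward or backward from the sign of current acceleration.
; Zero X acceleration leaves the facing unchanged.
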(event Input|EnhancedActionEvents|EnhancedInputActionIA_Move
  (params (ActionValue :type Float%20%28double-precision%29) (ElapsedSeconds :type Float%20%28double-precision%29) (TriggeredSeconds :type Float%20%28double-precision%29) (InputAction :type Input%20Action%20Object%20Reference :default "/Game/Input/IA_Move.IA_Move"))
  (CallFunction|RotateController)
  (Pawn|Input|AddMovementInput "1.000000,0.000000,0.000000" (Math|Conversions|ToFloat(Integer) (Math|Float|Round ActionValue)) false))

(event Input|EnhancedActionEvents|EnhancedInputActionIA_Jump
  (params (ActionValue :type Boolean) (ElapsedSeconds :type Float%20%28double-precision%29) (TriggeredSeconds :type Float%20%28double-precision%29) (InputAction :type Input%20Action%20Object%20Reference :default "/Game/Input/IA_Jump.IA_Jump"))
  (:Started
    (Character|Jump)))

(event EventBeginPlay
  (PlayerCharacterInput|PlayerCharacterInputMapping))

(fn ConstructionScript)

(fn PlayerCharacterInputMapping
  (bind _asplayer_controller (Utilities|Casting|CastToPlayerController (Pawn|GetController)))
  (Utilities|IsValid (PlayerController|LocalPlayerSubsystems|GetEnhancedInputLocalPlayerSubsystem _asplayer_controller)
    (:Is%20Valid
      (Input|AddMappingContext (PlayerController|LocalPlayerSubsystems|GetEnhancedInputLocalPlayerSubsystem _asplayer_controller) "/Game/Input/IMC_Saytr.IMC_Saytr" 0 "(bIgnoreAllPressedKeysUntilRelease=True,bForceImmediately=False,bNotifyUserSettings=False)"))))

(fn RotateController
  (bind _charactermovement (Variables|Character|GetCharacterMovement))
  (bind _returnvalue (Pawn|Components|CharacterMovement|GetCurrentAcceleration _charactermovement))
  (if (> (.x _returnvalue) 0.0)
    (Pawn|SetControlRotation (Pawn|GetController) (Math|Rotator|MakeRotator 0.0 0.0 0.0))
    (elif (< (.x _returnvalue) 0.0)
      (Pawn|SetControlRotation (Pawn|GetController) (Math|Rotator|MakeRotator 0.0 0.0 1.8e+02)))))